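; Orange fruit pickup for the arcade game that the player eats by touching it.
; On BeginPlay it spawns a scaled-up level-up particle burst at its collision location and plays a spawn sound.
; Overlap with BP_Player plays the eat sound, fires the eaten VFX and removes collision, meshes and glow at once, delaying actor destruction a few seconds.
; No score or player effect is applied in this Blueprint.
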(event `self.ReceiveBeginPlay`
  ;[0 1 0.1845] Goodie Spwan FX
  (`self.SpawnFX`))

(event `self.Collision.OnComponentBeginOverlap`
  (params (OverlappedComponent :type "PrimitiveComponent Object Reference") (OtherActor :type "Actor Object Reference") (OtherComp :type "PrimitiveComponent Object Reference") (OtherBodyIndex :type Integer) (bFromSweep :type Boolean) (SweepResult :type "HitResult Structure (by ref)"))
  (cast `/Game/ArcadeGame/Blueprints/Characters/BP_Player` OtherActor)
  (`|ExecutionSequence`
    (:`then_0`
      ;[0 1 0.2555] Fruit Eaten Handling
      (`GameplayStatics.PlaySound2D` "/Game/ArcadeGame/Audio/SFX_EatSpecial_Cue.SFX_EatSpecial_Cue" 1.0 1.0 0.0 null null)
      (`ActorComponent.Activate` (`self.VFX_Eaten`) false)
      (`ActorComponent.K2_DestroyComponent` (`self.Collision`))
      (`ActorComponent.K2_DestroyComponent` (`self.SM_Orange`))
      (`ActorComponent.K2_DestroyComponent` (`self.VFX_Glow`))
      (`ActorComponent.K2_DestroyComponent` (`self.SM_Leaf`))
      (`KismetSystemLibrary.Delay` 5.0)
      (`self.K2_DestroyActor`))))

(fn `SpawnFX`
  (bind _returnvalue (`GameplayStatics.SpawnEmitterAtLocation` "/Game/InfinityBladeEffects/Effects/FX_Mobile/Misc/P_levelUp.P_levelUp" (`SceneComponent.K2_GetComponentLocation` (`self.Collision`))))
  (`SceneComponent.SetWorldScale3D` _returnvalue (3.0 3.0 3.0))
  (`GameplayStatics.PlaySound2D` "/Game/ArcadeGame/Audio/SFX_FruitSpawn_Cue.SFX_FruitSpawn_Cue" 1.0 1.0 0.0 null null))

(fn `UserConstructionScript`)